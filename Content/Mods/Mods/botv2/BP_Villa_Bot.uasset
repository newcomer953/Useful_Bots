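; PAYDAY 3 mod actor for solo Villa heists that makes AI crew deliver carried bags to the escape van during loud phases.
; Looping timers mirror Botv1_5's Trigger, track crew positions and re-arm DoOnce gates.
; Carriers get Move_Stealth orders with Moveto_Loud behavior toward whichever preset point the van is near.
; On arrival, bags are secured, destroyed and respawned through a bag spawner created at the stopped van's trigger volume.
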(event Custom|The%20Start
  (bind _returnvalue (Class|SBZBagManager|Get))
  (bind _returnvalue_2 (Class|SBZBagManager|Get))
  (bind _returnvalue_3 (Class|SBZBagManager|Get))
  (bind _point_1 (Variables|Default|GetPoint%201))
  (bind _point_2 (Variables|Default|GetPoint%202))
  (bind _point_2_2 (Variables|Default|GetPoint%202))
  (bind _bagspawner (Variables|Default|GetBagSpawner))
  (bind _bagspawner_2 (Variables|Default|GetBagSpawner))
  (bind _bagspawner_3 (Variables|Default|GetBagSpawner))
  (bind _crew1_location (Variables|Default|GetCrew1_location))
  (bind _point_2_3 (Variables|Default|GetPoint%202))
  (bind _point_1_2 (Variables|Default|GetPoint%201))
  (bind _point_1_3 (Variables|Default|GetPoint%201))
  (bind _returnvalue_4 (Actor|GetActorOfClass "/Game/Mods/Mods/botv2/botv1_5.botv1_5_C"))
  (Variables|Default|SetTrigger (Variables|/Game/Mods/Mods/botv2/botv1_5.botv1_5_C|GetTrigger _returnvalue_4))
  (bind _aspd3heist_game_state (Utilities|Casting|CastToPD3HeistGameState (Class|SBZMissionState|GetSBZMissionState)))
  (if (== (Variables|Default|GetTrigger) 1)
    (if (Math|Boolean|ORBoolean (Utilities|Enum|Equal(Enum) (Class|PD3HeistGameState|GetCurrentHeistState _aspd3heist_game_state) "Anticipation") (Utilities|Enum|Equal(Enum) (Class|PD3HeistGameState|GetCurrentHeistState _aspd3heist_game_state) "Assault") (Utilities|Enum|Equal(Enum) (Class|PD3HeistGameState|GetCurrentHeistState _aspd3heist_game_state) "Control") (Utilities|Enum|Equal(Enum) (Class|PD3HeistGameState|GetCurrentHeistState _aspd3heist_game_state) "PointOfNoReturn"))
      (Utilities|FlowControl|Sequence
        (:then_0
          (bind _outactors (Actor|GetAllActorsOfClass "/Script/Starbreeze.SBZAICrewCharacter"))
          (bind _outactors_2 (Actor|GetAllActorsOfClass "/Game/Vehicle/_Mockup/Escape/BP_EscapeVan.BP_EscapeVan_C"))
          (for _array_element _outactors_2
            (Utilities|FlowControl|Sequence
              (:then_0
                (if (> (Utilities|Array|Length (Variables|/Script/Starbreeze.SBZCharacter|GetBagActorArray (Utilities|Array|Get(acopy) _outactors))) 0)
                  (Utilities|FlowControl|Sequence
                    (:then_0
                      (if (Utilities|IsValid (Variables|Default|GetBagSpawner))
                        (Utilities|FlowControl|Sequence
                          (:then_0
                            (if (< (Math|Vector|Distance(Vector) _point_1_3 (Transformation|GetActorLocation _array_element)) 5e+02)
                              (Variables|Default|SetCrewDestination _point_1_3)
                              (Utilities|FlowControl|DoOnce false :!label _label
                                (:Completed
                                  (bind _assbzaicrew_controller (Utilities|Casting|CastToSBZAICrewController (AI|GetAIController (Utilities|Array|Get(acopy) _outactors))))
                                  (bind _asmove_stealth (Utilities|Casting|CastToMove_Stealth (Class|SBZAILibrary|CreateAIOrder "/Game/Mods/Mods/botv2/Move_Stealth.Move_Stealth_C" _assbzaicrew_controller)))
                                  (if (or (Class|KismetMathLibrary|EqualExactlyVectorVector (Variables|Default|GetCrewDestination) _point_1_3) (Class|KismetMathLibrary|EqualExactlyVectorVector _point_2 _crew1_location))
                                    (Class|SBZAIOrderMoveto|SetMovetoLocation _asmove_stealth (Variables|Default|GetCrewDestination))
                                    (bind _output_get (Variables|/Script/Starbreeze.SBZAIController|SetCurrentOrder _assbzaicrew_controller _asmove_stealth))
                                    (Variables|/Script/Starbreeze.SBZAIOrder|SetBehavior _output_get "/Game/Mods/Mods/botv2/Moveto_Loud.Moveto_Loud"))))))
                          (:then_1
                            (if (< (Math|Vector|Distance(Vector) _point_2 (Transformation|GetActorLocation _array_element)) 5e+02)
                              (Variables|Default|SetCrewDestination _point_2)
                              (goto _label))))))
                    (:then_1
                      (if (and (<= (Math|Vector|Distance(Vector) (Variables|Default|GetCrewDestination) _crew1_location) 3e+02) (> (Utilities|Array|Length (Variables|/Script/Starbreeze.SBZCharacter|GetBagActorArray (Utilities|Array|Get(acopy) _outactors))) 0))
                        (Utilities|FlowControl|DoOnce false
                          (:Completed
                            (Class|SBZBagManager|SecureBag _returnvalue (Utilities|Array|Get(acopy) (Variables|/Script/Starbreeze.SBZCharacter|GetBagHandleArray (Utilities|Array|Get(acopy) _outactors))) false)
                            (bind _output_get_2 (Variables|Default|SetBag%20Type%201 (.BagType (Utilities|Struct|BreakSBZBagHandle (Utilities|Array|Get(acopy) (Variables|/Script/Starbreeze.SBZCharacter|GetBagHandleArray (Utilities|Array|Get(acopy) _outactors)))))))
                            (Variables|Default|SetOriginalBags (Variables|/Script/Starbreeze.SBZBagManager|GetBags _returnvalue))
                            (Variables|/Script/Starbreeze.SBZBagSpawner|SetBagTypeToSpawn _bagspawner_3 _output_get_2)
                            (Class|SBZBagSpawner|StartSpawningBags _bagspawner_3)
                            (Actor|DestroyActor (Utilities|Array|Get(acopy) (Variables|/Script/Starbreeze.SBZCharacter|GetBagActorArray (Utilities|Array|Get(acopy) _outactors))))
                            (Math|Integer|IncrementInt (Variables|Default|GetReset_destroy)
                              (:%20%20
                                (Utilities|FlowControl|Sequence
                                  (:then_0
                                    (CallFunction|ResetLoud)
                                    (Utilities|FlowControl|Sequence
                                      (:then_0
                                        (Utilities|Array|Clear (Variables|/Script/Starbreeze.SBZCharacter|GetBagActorArray (Utilities|Array|Get(acopy) _outactors)))
                                        (Utilities|Array|Clear (Variables|/Script/Starbreeze.SBZCharacter|GetBagHandleArray (Utilities|Array|Get(acopy) _outactors)))
                                        (Utilities|Array|Clear (Variables|/Script/Starbreeze.SBZCharacter|GetCurrentCarryTypeArray (Utilities|Array|Get(acopy) _outactors)))
                                        (CallFunction|PrinttoModLoader "Success 1")
                                        (Variables|/Script/Starbreeze.SBZBagManager|SetBags (Class|SBZBagManager|Get) (Variables|Default|GetOriginalBags))
                                        (Variables|/Script/Starbreeze.SBZAIController|SetCurrentOrder _assbzaicrew_controller 0))
                                      (:then_1
                                        (Variables|Default|SetReset_destroy 0))))
                                  (:then_1
                                    (CallFunction|ResetOrderLoud))))))))))))
              (:then_1
                (if (> (Utilities|Array|Length (Variables|/Script/Starbreeze.SBZCharacter|GetBagActorArray (Utilities|Array|Get(acopy) _outactors 1))) 0)
                  (Utilities|FlowControl|Sequence
                    (:then_0
                      (if (Utilities|IsValid (Variables|Default|GetBagSpawner))
                        (Utilities|FlowControl|Sequence
                          (:then_0
                            (if (< (Math|Vector|Distance(Vector) _point_1 (Transformation|GetActorLocation _array_element)) 5e+02)
                              (Variables|Default|SetCrewDestination _point_1)
                              (Utilities|FlowControl|DoOnce false :!label _label_2
                                (:Completed
                                  (bind _assbzaicrew_controller_2 (Utilities|Casting|CastToSBZAICrewController (AI|GetAIController (Utilities|Array|Get(acopy) _outactors 1))))
                                  (bind _asmove_stealth_2 (Utilities|Casting|CastToMove_Stealth (Class|SBZAILibrary|CreateAIOrder "/Game/Mods/Mods/botv2/Move_Stealth.Move_Stealth_C" _assbzaicrew_controller_2)))
                                  (if (or (Class|KismetMathLibrary|EqualExactlyVectorVector (Variables|Default|GetCrewDestination) _point_1) (Class|KismetMathLibrary|EqualExactlyVectorVector (Variables|Default|GetCrewDestination) _point_2_3))
                                    (Class|SBZAIOrderMoveto|SetMovetoLocation _asmove_stealth_2 (Variables|Default|GetCrewDestination))
                                    (bind _output_get_3 (Variables|/Script/Starbreeze.SBZAIController|SetCurrentOrder _assbzaicrew_controller_2 _asmove_stealth_2))
                                    (Variables|/Script/Starbreeze.SBZAIOrder|SetBehavior _output_get_3 "/Game/Mods/Mods/botv2/Moveto_Loud.Moveto_Loud"))))))
                          (:then_1
                            (if (< (Math|Vector|Distance(Vector) _point_2_3 (Transformation|GetActorLocation _array_element)) 5e+02)
                              (Variables|Default|SetCrewDestination _point_2_3)
                              (goto _label_2))))))
                    (:then_1
                      (if (and (<= (Math|Vector|Distance(Vector) (Variables|Default|GetCrewDestination) (Variables|Default|GetCrew2_location)) 3e+02) (> (Utilities|Array|Length (Variables|/Script/Starbreeze.SBZCharacter|GetBagActorArray (Utilities|Array|Get(acopy) _outactors 1))) 0))
                        (Utilities|FlowControl|DoOnce false
                          (:Completed
                            (Class|SBZBagManager|SecureBag _returnvalue_3 (Utilities|Array|Get(acopy) (Variables|/Script/Starbreeze.SBZCharacter|GetBagHandleArray (Utilities|Array|Get(acopy) _outactors 1))) false)
                            (bind _output_get_4 (Variables|Default|SetBag%20Type%202 (.BagType (Utilities|Struct|BreakSBZBagHandle (Utilities|Array|Get(acopy) (Variables|/Script/Starbreeze.SBZCharacter|GetBagHandleArray (Utilities|Array|Get(acopy) _outactors 1)))))))
                            (Variables|Default|SetOriginalBags (Variables|/Script/Starbreeze.SBZBagManager|GetBags _returnvalue_3))
                            (Variables|/Script/Starbreeze.SBZBagSpawner|SetBagTypeToSpawn _bagspawner_2 _output_get_4)
                            (Class|SBZBagSpawner|StartSpawningBags _bagspawner_2)
                            (Actor|DestroyActor (Utilities|Array|Get(acopy) (Variables|/Script/Starbreeze.SBZCharacter|GetBagActorArray (Utilities|Array|Get(acopy) _outactors 1))))
                            (Math|Integer|IncrementInt (Variables|Default|GetReset_destroy)
                              (:%20%20
                                (Utilities|FlowControl|Sequence
                                  (:then_0
                                    (CallFunction|ResetLoud)
                                    (Utilities|FlowControl|Sequence
                                      (:then_0
                                        (Utilities|Array|Clear (Variables|/Script/Starbreeze.SBZCharacter|GetBagActorArray (Utilities|Array|Get(acopy) _outactors 1)))
                                        (Utilities|Array|Clear (Variables|/Script/Starbreeze.SBZCharacter|GetBagHandleArray (Utilities|Array|Get(acopy) _outactors 1)))
                                        (Utilities|Array|Clear (Variables|/Script/Starbreeze.SBZCharacter|GetCurrentCarryTypeArray (Utilities|Array|Get(acopy) _outactors 1)))
                                        (CallFunction|PrinttoModLoader "Success 2")
                                        (Variables|/Script/Starbreeze.SBZBagManager|SetBags (Class|SBZBagManager|Get) (Variables|Default|GetOriginalBags))
                                        (Variables|/Script/Starbreeze.SBZAIController|SetCurrentOrder _assbzaicrew_controller_2 0))
                                      (:then_1
                                        (Variables|Default|SetReset_destroy 0))))
                                  (:then_1
                                    (CallFunction|ResetOrderLoud))))))))))))
              (:then_2
                (if (> (Utilities|Array|Length (Variables|/Script/Starbreeze.SBZCharacter|GetBagActorArray (Utilities|Array|Get(acopy) _outactors 2))) 0)
                  (Utilities|FlowControl|Sequence
                    (:then_0
                      (if (Utilities|IsValid (Variables|Default|GetBagSpawner))
                        (Utilities|FlowControl|Sequence
                          (:then_0
                            (if (< (Math|Vector|Distance(Vector) _point_1_2 (Transformation|GetActorLocation _array_element)) 5e+02)
                              (Variables|Default|SetCrewDestination _point_1_2)
                              (Utilities|FlowControl|DoOnce false :!label _label_3
                                (:Completed
                                  (bind _assbzaicrew_controller_3 (Utilities|Casting|CastToSBZAICrewController (AI|GetAIController (Utilities|Array|Get(acopy) _outactors 2))))
                                  (bind _asmove_stealth_3 (Utilities|Casting|CastToMove_Stealth (Class|SBZAILibrary|CreateAIOrder "/Game/Mods/Mods/botv2/Move_Stealth.Move_Stealth_C" _assbzaicrew_controller_3)))
                                  (if (or (Class|KismetMathLibrary|EqualExactlyVectorVector (Variables|Default|GetCrewDestination) _point_1_2) (Class|KismetMathLibrary|EqualExactlyVectorVector (Variables|Default|GetCrewDestination) _point_2_2))
                                    (Class|SBZAIOrderMoveto|SetMovetoLocation _asmove_stealth_3 (Variables|Default|GetCrewDestination))
                                    (bind _output_get_5 (Variables|/Script/Starbreeze.SBZAIController|SetCurrentOrder _assbzaicrew_controller_3 _asmove_stealth_3))
                                    (Variables|/Script/Starbreeze.SBZAIOrder|SetBehavior _output_get_5 "/Game/Mods/Mods/botv2/Moveto_Loud.Moveto_Loud"))))))
                          (:then_1
                            (if (< (Math|Vector|Distance(Vector) _point_2_2 (Transformation|GetActorLocation _array_element)) 5e+02)
                              (Variables|Default|SetCrewDestination _point_2_2)
                              (goto _label_3))))))
                    (:then_1
                      (if (and (<= (Math|Vector|Distance(Vector) (Variables|Default|GetCrewDestination) (Variables|Default|GetCrew3_location)) 3e+02) (> (Utilities|Array|Length (Variables|/Script/Starbreeze.SBZCharacter|GetBagActorArray (Utilities|Array|Get(acopy) _outactors 2))) 0))
                        (Utilities|FlowControl|DoOnce false
                          (:Completed
                            (Class|SBZBagManager|SecureBag _returnvalue_2 (Utilities|Array|Get(acopy) (Variables|/Script/Starbreeze.SBZCharacter|GetBagHandleArray (Utilities|Array|Get(acopy) _outactors 2))) false)
                            (bind _output_get_6 (Variables|Default|SetBag%20Type%203 (.BagType (Utilities|Struct|BreakSBZBagHandle (Utilities|Array|Get(acopy) (Variables|/Script/Starbreeze.SBZCharacter|GetBagHandleArray (Utilities|Array|Get(acopy) _outactors 2)))))))
                            (Variables|Default|SetOriginalBags (Variables|/Script/Starbreeze.SBZBagManager|GetBags _returnvalue_2))
                            (Variables|/Script/Starbreeze.SBZBagSpawner|SetBagTypeToSpawn _bagspawner _output_get_6)
                            (Class|SBZBagSpawner|StartSpawningBags _bagspawner)
                            (Actor|DestroyActor (Utilities|Array|Get(acopy) (Variables|/Script/Starbreeze.SBZCharacter|GetBagActorArray (Utilities|Array|Get(acopy) _outactors 2))))
                            (Math|Integer|IncrementInt (Variables|Default|GetReset_destroy)
                              (:%20%20
                                (Utilities|FlowControl|Sequence
                                  (:then_0
                                    (CallFunction|ResetLoud)
                                    (Utilities|FlowControl|Sequence
                                      (:then_0
                                        (Utilities|Array|Clear (Variables|/Script/Starbreeze.SBZCharacter|GetBagActorArray (Utilities|Array|Get(acopy) _outactors 2)))
                                        (Utilities|Array|Clear (Variables|/Script/Starbreeze.SBZCharacter|GetBagHandleArray (Utilities|Array|Get(acopy) _outactors 2)))
                                        (Utilities|Array|Clear (Variables|/Script/Starbreeze.SBZCharacter|GetCurrentCarryTypeArray (Utilities|Array|Get(acopy) _outactors 2)))
                                        (CallFunction|PrinttoModLoader "Success 3")
                                        (Variables|/Script/Starbreeze.SBZBagManager|SetBags (Class|SBZBagManager|Get) (Variables|Default|GetOriginalBags))
                                        (Variables|/Script/Starbreeze.SBZAIController|SetCurrentOrder _assbzaicrew_controller_3 0))
                                      (:then_1
                                        (Variables|Default|SetReset_destroy 0))))
                                  (:then_1
                                    (CallFunction|ResetOrderLoud)))))))))))))))
        (:then_1
          (CallFunction|FindLootTriggerVan))))))

(event Custom|CheckTrigger
  (bind _trigger (Variables|Default|GetTrigger))
  (if (== _trigger 0)
    (CallFunction|ResetLoud)
    (CallFunction|ResetOrderLoud)
    (Variables|Default|SetReset_destroy 0)
    (Utilities|FlowControl|DoOnce false :!label _label
      (:Completed
        (bind _outactors (Actor|GetAllActorsOfClass "/Script/Starbreeze.SBZAICrewController"))
        (for _array_element _outactors
          (Variables|/Script/Starbreeze.SBZAIController|SetCurrentOrder _array_element 0))))
    (elif (== _trigger 1)
      (goto _label Reset))))

(event Custom|FindLootTriggerVan
  (bind _outactors (Actor|GetAllActorsOfClass "/Game/Vehicle/_Mockup/Escape/BP_EscapeVan.BP_EscapeVan_C"))
  (for _array_element _outactors
    (bind _outactors_2 (Actor|GetAllActorsOfClass "/Script/Starbreeze.SBZBagTriggerVolume"))
    (for _array_element_2 _outactors_2
      (if (< (Math|Vector|Distance(Vector) (Transformation|GetActorLocation _array_element_2) (Transformation|GetActorLocation _array_element)) 4e+02)
        (if (Class|SBZVehicleSplineFollowingComponent|IsStopped (Variables|/Script/Starbreeze.SBZWheeledVehicle|GetSplineFollowingComponent _array_element))
          (Variables|Default|SetBagTriggerLocationVan (Transformation|GetActorLocation _array_element_2))
          (Utilities|FlowControl|DoOnce false :!label _label
            (:Completed
              (bind _returnvalue (Game|SpawnActorfromClass "/Script/Starbreeze.SBZBagSpawner" (Math|Transform|MakeTransform (Variables|Default|GetBagTriggerLocationVan)) "AlwaysSpawn" 0 0))
              (Variables|Default|SetBagSpawner _returnvalue)
              (CallFunction|PrinttoModLoader "SPAWNED BAG SPAWNER")))
          (else
            (CallFunction|PrinttoModLoader "Helicopter is near but not stopped at bag trigger volume")
            (Actor|DestroyActor (Variables|Default|GetBagSpawnerHelicopter))
            (goto _label Reset)))))))

(event Custom|Reset%20the%20Reset%201
  (bind _outactors (Actor|GetAllActorsOfClass "/Script/Starbreeze.SBZAICrewCharacter"))
  (bind _assbzaicrew_controller (Utilities|Casting|CastToSBZAICrewController (AI|GetAIController (Utilities|Array|Get(acopy) _outactors))))
  (if (Math|Boolean|ANDBoolean (!= (Variables|/Script/Starbreeze.SBZAIController|GetCurrentOrder _assbzaicrew_controller) "/Game/Mods/Mods/botv2/Move_Stealth.Move_Stealth") (== (Variables|Default|GetTrigger) 1) (> (Utilities|Array|Length (Variables|/Script/Starbreeze.SBZCharacter|GetBagActorArray (Utilities|Array|Get(acopy) _outactors))) 0))
    (CallFunction|ResetOrderLoud)))

(event Custom|Reset%20the%20Reset%202
  (bind _outactors (Actor|GetAllActorsOfClass "/Script/Starbreeze.SBZAICrewCharacter"))
  (bind _assbzaicrew_controller (Utilities|Casting|CastToSBZAICrewController (AI|GetAIController (Utilities|Array|Get(acopy) _outactors 1))))
  (if (Math|Boolean|ANDBoolean (!= (Variables|/Script/Starbreeze.SBZAIController|GetCurrentOrder _assbzaicrew_controller) "/Game/Mods/Mods/botv2/Move_Stealth.Move_Stealth") (== (Variables|Default|GetTrigger) 1) (> (Utilities|Array|Length (Variables|/Script/Starbreeze.SBZCharacter|GetBagActorArray (Utilities|Array|Get(acopy) _outactors 1))) 0))
    (CallFunction|ResetOrderLoud)))

(event Custom|Reset%20Loud
  (bind _returnvalue (Class|SBZBagManager|Get))
  (bind _returnvalue_2 (Class|SBZBagManager|Get))
  (bind _returnvalue_3 (Class|SBZBagManager|Get))
  (bind _bagspawner (Variables|Default|GetBagSpawner))
  (bind _bagspawner_2 (Variables|Default|GetBagSpawner))
  (bind _bagspawner_3 (Variables|Default|GetBagSpawner))
  (Utilities|FlowControl|Sequence
    (:then_0
      (Utilities|FlowControl|DoOnce false) ; enters at Reset
    )
    (:then_1
      (Utilities|FlowControl|DoOnce false) ; enters at Reset
    )
    (:then_2
      (Utilities|FlowControl|DoOnce false) ; enters at Reset
    )))

(event Custom|SetCrews
  (bind _outactors (Actor|GetAllActorsOfClass "/Script/Starbreeze.SBZAICrewCharacter"))
  (Variables|Default|SetCrews _outactors))

(event Custom|Crewlocation
  (bind _outactors (Actor|GetAllActorsOfClass "/Script/Starbreeze.SBZAICrewCharacter"))
  (for (_array_element _array_index) _outactors
    (Utilities|FlowControl|Sequence
      (:then_0
        (if (== _array_index 0)
          (Variables|Default|SetCrew1_location (Transformation|GetActorLocation _array_element))))
      (:then_1
        (if (== _array_index 1)
          (Variables|Default|SetCrew2_location (Transformation|GetActorLocation _array_element))))
      (:then_2
        (if (== _array_index 2)
          (Variables|Default|SetCrew3_location (Transformation|GetActorLocation _array_element)))))))

(event Custom|Reset%20Order%20Loud
  (bind _crewdestination (Variables|Default|GetCrewDestination))
  (bind _crewdestination_2 (Variables|Default|GetCrewDestination))
  (bind _crewdestination_3 (Variables|Default|GetCrewDestination))
  (Utilities|FlowControl|Sequence
    (:then_0
      (Utilities|FlowControl|DoOnce false) ; enters at Reset
    )
    (:then_1
      (Utilities|FlowControl|DoOnce false) ; enters at Reset
    )
    (:then_2
      (Utilities|FlowControl|DoOnce false) ; enters at Reset
    )))

(event Custom|Reset%20the%20Reset%203
  (bind _outactors (Actor|GetAllActorsOfClass "/Script/Starbreeze.SBZAICrewCharacter"))
  (bind _assbzaicrew_controller (Utilities|Casting|CastToSBZAICrewController (AI|GetAIController (Utilities|Array|Get(acopy) _outactors 2))))
  (if (Math|Boolean|ANDBoolean (!= (Variables|/Script/Starbreeze.SBZAIController|GetCurrentOrder _assbzaicrew_controller) "/Game/Mods/Mods/botv2/Move_Stealth.Move_Stealth") (== (Variables|Default|GetTrigger) 1) (> (Utilities|Array|Length (Variables|/Script/Starbreeze.SBZCharacter|GetBagActorArray (Utilities|Array|Get(acopy) _outactors 2))) 0))
    (CallFunction|ResetOrderLoud)))

(event EventBeginPlay
  (bind _returnvalue (Game|GetCurrentLevelName true))
  (if (and (Class|SBZOnlineFunctionLibrary|IsSoloGame) (Utilities|Enum|Equal(Enum) _returnvalue "Villa"))
    (Utilities|FlowControl|Sequence
      (:then_0
        (Input|EnableInput (Game|GetPlayerController 0)))
      (:then_1
        (Utilities|Time|SetTimerbyFunctionName 0 "The Start" 0.2 true))
      (:then_2
        (Utilities|Time|SetTimerbyFunctionName 0 "Crewlocation" 0.2 true))
      (:then_3
        (Utilities|Time|SetTimerbyFunctionName 0 "SetCrews" 0.2))
      (:then_4
        (Utilities|Time|SetTimerbyFunctionName 0 "Reset the Reset 1" 0.3 true))
      (:then_5
        (Utilities|Time|SetTimerbyFunctionName 0 "Reset the Reset 2" 0.3 true))
      (:then_6
        (Utilities|Time|SetTimerbyFunctionName 0 "Reset the Reset 3" 0.3 true))
      (:then_7
        (Utilities|Time|SetTimerbyFunctionName 0 "CheckTrigger" 0.2 true)))))

(fn ConstructionScript
  (|CallParentFunction))